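; Demo room sphere actor for GFur fur, with flag-gated showcases that all launch from BeginPlay.
; Timelines bob the actor along X from its start position and drive three skeletal morph targets.
; A delay loop alternates visibility between two GFur components every two seconds, reusing its enable flag as toggle state.
; The swap option destroys the first fur component once and adds a replacement with a different grow mesh, material and fur settings.
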(event `self.ReceiveBeginPlay`
  (bind _skeletalmeshcomponent (`self.SkeletalMeshComponent`))
  (`|ExecutionSequence`
    (:`then_0`
      ;[1 1 1] Animation of the sphere
      (if (`self.AnimatePosition`)
        (set `self.DefaultPosition` (`self.K2_GetActorLocation`))
        (bind (_direction _position) (`Timeline|Timeline_1`)
          (:`Update`
            (`self.K2_SetActorRelativeLocation` (+ (`self.DefaultPosition`) (`KismetMathLibrary.VLerp` (0.0 0.0 0.0) (25.0 0.0 0.0) _position)))))))
    (:`then_1`
      ;[1 1 1] Morph targets
      (if (`self.PlayMorphTargets`)
        (bind (_direction_2 _track_1 _track_2 _track_3) (`Timeline|Timeline_0`)
          (:`Update`
            (`SkeletalMeshComponent.SetMorphTarget` _skeletalmeshcomponent "Sphere_Morph_1" _track_1 true)
            (`SkeletalMeshComponent.SetMorphTarget` _skeletalmeshcomponent "Sphere_Morph_2" _track_2 true)
            (`SkeletalMeshComponent.SetMorphTarget` _skeletalmeshcomponent "Sphere_Morph_3" _track_3 true)))))
    (:`then_2`
      ;[1 1 1] Changing fur components via visibility
      (if (`self.Visibility`)
        (`KismetSystemLibrary.Delay` 2.0 :!label _label)
        (`SceneComponent.SetVisibility` (`self.GFur_1`) (`self.Visibility`) false)
        (`SceneComponent.SetVisibility` (`self.GFur_2`) (not (`self.Visibility`)) false)
        (set `self.Visibility` (not (`self.Visibility`)))
        (goto _label)))
    (:`then_3`
      ;[1 1 1] Changing fur components by destroying and creating new one
      (if (`self.Swap Components`)
        (`KismetSystemLibrary.Delay` 1.0)
        (`ActorComponent.K2_DestroyComponent` (`self.GFur_1`))
        (bind _returnvalue (`AddComponent|NODE_AddGFurComponent-0`))
        (`|ExecutionSequence`
          (:`then_0`
            (set `GFurComponent.SkeletalGrowMesh` "/GFur/gFurPRO/DemoRoom/Sphere/Fur/Sphere_GrowMesh_Stripe.Sphere_GrowMesh_Stripe" _returnvalue))
          (:`then_1`
            (`PrimitiveComponent.SetMaterial` _returnvalue 0 "/GFur/gFurPRO/DemoRoom/Sphere/Fur/Sphere_Fur_Red_Material.Sphere_Fur_Red_Material"))
          (:`then_2`
            (set `GFurComponent.FurLength` 30.0 _returnvalue))
          (:`then_3`
            (set `GFurComponent.LayerCount` 64 _returnvalue)))))))

(fn `UserConstructionScript`)