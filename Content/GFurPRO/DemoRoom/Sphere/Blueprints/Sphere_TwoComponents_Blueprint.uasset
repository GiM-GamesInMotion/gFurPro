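; Demo sphere actor from the GFurPRO demo room that animates a skeletal mesh's shape and the actor's position.
; On BeginPlay, two optional flags independently start timelines.
; PlayMorphTargets drives three sphere morph targets from separate tracks of one timeline.
; AnimatePosition caches the starting location, then uses another timeline to lerp a small X-axis offset from it.
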(event `self.ReceiveBeginPlay`
  (bind _skeletalmeshcomponent (`self.SkeletalMeshComponent`))
  (`|ExecutionSequence`
    (:`then_0`
      (if (`self.PlayMorphTargets`)
        (bind (_direction _track_1 _track_2 _track_3) (`Timeline|Timeline_0`)
          (:`Update`
            (`SkeletalMeshComponent.SetMorphTarget` _skeletalmeshcomponent "Sphere_Morph_1" _track_1 true)
            (`SkeletalMeshComponent.SetMorphTarget` _skeletalmeshcomponent "Sphere_Morph_2" _track_2 true)
            (`SkeletalMeshComponent.SetMorphTarget` _skeletalmeshcomponent "Sphere_Morph_3" _track_3 true)))))
    (:`then_1`
      (if (`self.AnimatePosition`)
        (set `self.DefaultPosition` (`self.K2_GetActorLocation`))
        (bind (_direction_2 _position) (`Timeline|Timeline_1`)
          (:`Update`
            (`self.K2_SetActorRelativeLocation` (+ (`self.DefaultPosition`) (`KismetMathLibrary.VLerp` (0.0 0.0 0.0) (25.0 0.0 0.0) _position)))))))))

(fn `UserConstructionScript`)